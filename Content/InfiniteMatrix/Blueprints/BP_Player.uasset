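; BP_Player is the player in InfiniteMatrix, constantly moving forward and steered sideways and vertically until dead.
; Tick pushes the actor along world X at MoveForward speed with a swept offset.
; MoveRight and MoveUp axes, noted as mouse control, add MoveSpeed-scaled movement input, then immediately consume it as a delta-time-scaled, swept local offset.
; IsDead gates all movement but is not set in these graphs.
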(event EventTick
  (params (DeltaSeconds :type Float%20%28single-precision%29))
  ;[1 1 1] Постоянное движение игрока вперед до столкновения
  (if (not (Variables|Default|GetIsDead))
    (Transformation|AddActorWorldOffset (Math|Vector|MakeVector (* DeltaSeconds (Variables|Default|GetMoveForward)) 0.0 0.0) true)))

(event Input|AxisEvents|InputAxisMoveRight
  (params (AxisValue :type Float%20%28single-precision%29))
  ;[1 1 1] Упрaвление игроком мышью
  (if (not (Variables|Default|GetIsDead))
    (Pawn|Input|AddMovementInput (Transformation|GetActorRightVector) (* AxisValue (Variables|Default|GetMoveSpeed)) false)
    (bind _returnvalue (Class|Pawn|ConsumeMovementInputVector))
    (Transformation|AddActorLocalOffset (* _returnvalue (Utilities|Time|GetWorldDeltaSeconds)) true false)))

(event Input|AxisEvents|InputAxisMoveUp
  (params (AxisValue :type Float%20%28single-precision%29))
  ;[1 1 1] Упрaвление игроком мышью
  (if (not (Variables|Default|GetIsDead))
    (Pawn|Input|AddMovementInput (Transformation|GetActorUpVector) (* AxisValue (Variables|Default|GetMoveSpeed)) false)
    (bind _returnvalue (Class|Pawn|ConsumeMovementInputVector))
    (Transformation|AddActorLocalOffset (* _returnvalue (Utilities|Time|GetWorldDeltaSeconds)) true false)))

(fn ConstructionScript)