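; Main menu level manager that switches between the main, options and highscore menu widgets.
; BeginPlay creates all three widgets with a back-reference to itself, shows the main menu and enables cursor and game-and-UI input.
; It also applies music and sound volumes from the settings save through sound mix class overrides.
; An IsInMenu flag tracks submenus, letting Escape clear widgets and restore the main menu.
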(event EventBeginPlay
  (bind _returnvalue (Game|GetPlayerController 0))
  (bind _save_slot_settings (Variables|Default|Getsave_slot_settings))
  (Utilities|FlowControl|Sequence
    (:then_0
      (bind _returnvalue_2 (UserInterface|CreateWidget "/Game/InfiniteMatrix/UI/WBP_MainMenu.WBP_MainMenu_C"))
      (Variables|/Game/InfiniteMatrix/UI/WBP_MainMenu.WBP_MainMenu_C|SetRefMainLevelManagerForMainMenu _returnvalue_2 self)
      (bind _output_get (Variables|Default|SetMainMenuWidget _returnvalue_2))
      (UserInterface|Viewport|AddtoViewport _output_get 0)
      (bind _returnvalue_3 (UserInterface|CreateWidget "/Game/InfiniteMatrix/UI/WBP_OptionsMenu.WBP_OptionsMenu_C"))
      (Variables|/Game/InfiniteMatrix/UI/WBP_OptionsMenu.WBP_OptionsMenu_C|SetRef_MainLevelManagerForOptionsMenu _returnvalue_3 self)
      (Variables|Default|SetOptionsWidget _returnvalue_3)
      (bind _returnvalue_4 (UserInterface|CreateWidget "/Game/InfiniteMatrix/UI/WBP_HighscoreMenu.WBP_HighscoreMenu_C"))
      (Variables|/Game/InfiniteMatrix/UI/WBP_HighscoreMenu.WBP_HighscoreMenu_C|SetRef_MainLevelManagerForHighscoreMenu _returnvalue_4 self)
      (Variables|Default|SetHighscoreWidget _returnvalue_4)
      (Input|SetInputModeGameandUI _returnvalue 0 "DoNotLock" true)
      (Variables|/Script/Engine.PlayerController|SetbShowMouseCursor _returnvalue true))
    (:then_1
      ;[1 1 1] Загружаем настройки звуков и музыки и применяем их для этого уровня (MainLevel)
      (Class|GameplayStatics|SetBaseSoundMix "/Game/InfiniteMatrix/Sounds/S_Volume_Mix.S_Volume_Mix")
      (bind _returnvalue_5 (SaveGame|DoesSaveGameExist _save_slot_settings))
      (if _returnvalue_5
        (bind _returnvalue_6 (SaveGame|LoadGamefromSlot _save_slot_settings))
        (else
          (SaveGame|CreateSaveGameObject "/Game/InfiniteMatrix/Blueprints/BP_SettingsSave.BP_SettingsSave_C")))
      (bind _asbp_settings_save (Utilities|Casting|CastToBP_SettingsSave _returnvalue_6))
      (Audio|SetSoundMixClassOverride "/Game/InfiniteMatrix/Sounds/S_Volume_Mix.S_Volume_Mix" "/Game/InfiniteMatrix/Sounds/S_Music_Class.S_Music_Class" (Variables|/Game/InfiniteMatrix/Blueprints/BP_SettingsSave.BP_SettingsSave_C|GetVolumeMusic _asbp_settings_save) 1.0 0.0 true)
      (Audio|SetSoundMixClassOverride "/Game/InfiniteMatrix/Sounds/S_Volume_Mix.S_Volume_Mix" "/Game/InfiniteMatrix/Sounds/S_Sounds_Class.S_Sounds_Class" (Variables|/Game/InfiniteMatrix/Blueprints/BP_SettingsSave.BP_SettingsSave_C|GetVolumeSounds _asbp_settings_save) 1.0 0.0 true))))

(event Input|KeyboardEvents|Escape
  (params (Key :type Key%20Structure :default "None"))
  (:Pressed
    (if (Variables|Default|GetIsInMenu)
      (Development|PrintString "true")
      (else
        (Development|PrintString "false")
        (CallFunction|BacktoMenu)))))

(fn ConstructionScript)

(fn OpenOptions
  (bind _optionswidget (Variables|Default|GetOptionsWidget))
  (UserInterface|Viewport|AddtoViewport _optionswidget 0)
  (Variables|/Game/InfiniteMatrix/UI/WBP_OptionsMenu.WBP_OptionsMenu_C|SetIsMainMenu _optionswidget true)
  (Variables|Default|SetIsInMenu false))

(fn OpenHighscoreMenu
  (UserInterface|Viewport|AddtoViewport (Variables|Default|GetHighscoreWidget) 0)
  (Variables|Default|SetIsInMenu false))

(fn BacktoMenu
  (bind _mainmenuwidget (Variables|Default|GetMainMenuWidget))
  (Viewport|RemoveAllWidgets)
  (UserInterface|Viewport|AddtoViewport _mainmenuwidget 0)
  (Default|SetButtonsVisibility _mainmenuwidget "Visible")
  (Variables|Default|SetIsInMenu true))

(fn RemoveWidgets
  (Widget|RemovefromParent (Variables|Default|GetMainMenuWidget))
  (Widget|RemovefromParent (Variables|Default|GetOptionsWidget))
  (Widget|RemovefromParent (Variables|Default|GetHighscoreWidget)))