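; BP_TunnelSpawner builds the chain of BP_Tunnel segments that the player travels through and registers itself with BP_GameManager on BeginPlay.
; Each new tunnel receives a spawner reference and rotation speed, then randomizes its wall.
; Later tunnels attach at the previous one's SpawnPoint and increment the score.
; SpawnSeveralTunnels handles restarts by destroying all tunnels, seeding a short chain from the player's location and resetting the score.
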(event EventBeginPlay
  ;[1 1 1] задаем ссылку на этот tunnelSpawner для GameManager
  (bind _outactors (Actor|GetAllActorsOfClass "/Game/InfiniteMatrix/Blueprints/BP_GameManager.BP_GameManager_C"))
  (Variables|/Game/InfiniteMatrix/Blueprints/BP_GameManager.BP_GameManager_C|SetRef_BPTunnelSpawner_BPGameManager (Utilities|Array|Get(acopy) _outactors) self))

(fn ConstructionScript)

(fn SpawnTunnel
  (params (Location :type Vector))
  ;[1 1 1] Спавн туннеля в переданных координатах, сохранения туннеля в переменной и задание для него ссылки для BP_Tunnel, добавление стенки
  (bind _returnvalue (Game|SpawnActorfromClass "/Game/InfiniteMatrix/Blueprints/BP_Tunnel.BP_Tunnel_C" (Math|Transform|MakeTransform Location "0, 0, 0" "1,1,1") "Undefined" 0 0))
  (bind _output_get (Variables|Default|SetLatestTunnel _returnvalue))
  (Variables|/Game/InfiniteMatrix/Blueprints/BP_Tunnel.BP_Tunnel_C|SetRef_BP_TunnelSpawner _output_get self)
  (Variables|/Game/InfiniteMatrix/Blueprints/BP_Tunnel.BP_Tunnel_C|SetRotateSpeed _output_get (Variables|Default|GetRotateSpeedForTunnel))
  (Default|RandomizeWall _output_get))

(fn SpawnTunnelatSpawnPoint
  ;[1 1 1] Спавн след. туннеля после прохода через триггер зону используя пред. туннель. увеличение счета
  (CallFunction|SpawnTunnel (Transformation|GetWorldLocation (Variables|/Game/InfiniteMatrix/Blueprints/BP_Tunnel.BP_Tunnel_C|GetSpawnPoint (Variables|Default|GetLatestTunnel))))
  (Default|IncrementScore (Variables|Default|GetRef_GameManager_BPTunnelSpawner)))

(fn SpawnSeveralTunnels
  (Utilities|FlowControl|Sequence
    (:then_0
      ;[1 1 1] Сброс счета (после рестарта сбрасываем скорость)
      (Default|ResetScore (Variables|Default|GetRef_GameManager_BPTunnelSpawner)))
    (:then_1
      ;[1 1 1] Удаление всех туннелей с уровня
      (bind _outactors (Actor|GetAllActorsOfClass "/Game/InfiniteMatrix/Blueprints/BP_Tunnel.BP_Tunnel_C"))
      (for _array_element _outactors
        (Actor|DestroyActor _array_element)))
    (:then_2
      ;[1 1 1] Спавн нескольких туннелей: первый туннель спавнится в месте положения игрока, остальные спавнятся в спавн поинте каждого предыдущего туннеля
      (for _index (range 0 2)
        (Utilities|IsValid (Variables|Default|GetLatestTunnel)
          (:Is%20Valid
            (CallFunction|SpawnTunnelatSpawnPoint))
          (:Is%20Not%20Valid
            (CallFunction|SpawnTunnel (Transformation|GetActorLocation (Game|Player|GetPlayerPawn 0)))))))
    (:then_3
      ;[1 1 1] После создания первых туннелей, обнуляем score
      (Default|ResetScore (Variables|Default|GetRef_GameManager_BPTunnelSpawner)))))