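; Game manager for a tunnel-running game, handling score, levels, pause, restart and game over.
; On BeginPlay it creates the HUD and menu widgets, starts tunnel spawning, loads highscore and volume saves, and binds the player's wall hit to GameOver.
; Scoring past a growing threshold raises the level, player speed and tunnel rotation.
; Pause freezes player and tunnels via IsDead and zeroed RotateSpeed; GameOver inserts the run into score-sorted saved records.
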(event Custom|CustomEvent_0
  ;[1 1 1] Биндим эвент у игрока когда он столкнется со стеной с функцией вызова геймовера
  (CallFunction|GameOver))

(event EventBeginPlay
  (bind _returnvalue (Game|GetPlayerController 0))
  (bind _save_slot_highscore (Variables|Default|Getsave_slot_highscore))
  (bind _save_slot_settings (Variables|Default|Getsave_slot_settings))
  (Utilities|FlowControl|Sequence
    (:then_0
      ;[1 1 1] Убираешь курсор мыши, включаем режим управления и сохраняем ссылку на игрока в переменной Player
      (Input|SetInputModeGameOnly _returnvalue)
      (Variables|/Script/Engine.PlayerController|SetbShowMouseCursor _returnvalue false)
      (bind _asbp_player (Utilities|Casting|CastToBP_Player (Game|Player|GetPlayerPawn 0)))
      (Variables|Default|SetPlayer _asbp_player))
    (:then_1
      ;[1 1 1] Создаем выджеты (options, pause menu, game over menu), задаем в них ссылки на GameManager
      (bind _returnvalue_2 (UserInterface|CreateWidget "/Game/InfiniteMatrix/UI/WBP_PauseMenu.WBP_PauseMenu_C"))
      (Variables|/Game/InfiniteMatrix/UI/WBP_PauseMenu.WBP_PauseMenu_C|SetRefGameManagerForPauseMenu _returnvalue_2 self)
      (Variables|Default|SetPauseWidget _returnvalue_2)
      (bind _returnvalue_3 (UserInterface|CreateWidget "/Game/InfiniteMatrix/UI/WBP_OptionsMenu.WBP_OptionsMenu_C"))
      (Variables|/Game/InfiniteMatrix/UI/WBP_OptionsMenu.WBP_OptionsMenu_C|SetRefGameManagerForOptionsMenu _returnvalue_3 self)
      (Variables|Default|SetOptionsWidget _returnvalue_3)
      (bind _returnvalue_4 (UserInterface|CreateWidget "/Game/InfiniteMatrix/UI/WBP_GameOverMenu.WBP_GameOverMenu_C"))
      (Variables|/Game/InfiniteMatrix/UI/WBP_GameOverMenu.WBP_GameOverMenu_C|SetRefGamaManagerForGameOverMenu _returnvalue_4 self)
      (Variables|Default|SetGameOverWidget _returnvalue_4))
    (:then_2
      ;[1 1 1] Создаем виджет со счетом, задание ссылки для виджета, сохранение виджета в переенной и инициализация текста в виджете нулем
      (bind _returnvalue_5 (UserInterface|CreateWidget "/Game/InfiniteMatrix/UI/WBP_Scores.WBP_Scores_C"))
      (UserInterface|Viewport|AddtoViewport _returnvalue_5 0)
      (Variables|/Game/InfiniteMatrix/UI/WBP_Scores.WBP_Scores_C|SetRef_GameManager_WBPScores _returnvalue_5 self)
      (bind _output_get (Variables|Default|SetHUD_Widget _returnvalue_5))
      (Default|UpdateScore _output_get))
    (:then_3
      ;[1 1 1] Задаем ссылку для BP_TunnelSpawner и первый вызов спавна туннелей в начале игры
      (bind _outactors (Actor|GetAllActorsOfClass "/Game/InfiniteMatrix/Blueprints/BP_TunnelSpawner.BP_TunnelSpawner_C"))
      (Variables|/Game/InfiniteMatrix/Blueprints/BP_TunnelSpawner.BP_TunnelSpawner_C|SetRef_GameManager_BPTunnelSpawner (Utilities|Array|Get(acopy) _outactors) self)
      (Default|SpawnSeveralTunnels (Utilities|Array|Get(acopy) _outactors)))
    (:then_4
      ;[1 1 1] создаем объект с сохранением, загружаем пред. рекорд и отображаем
      (bind _returnvalue_6 (SaveGame|DoesSaveGameExist _save_slot_highscore))
      (if _returnvalue_6
        (bind _returnvalue_7 (SaveGame|LoadGamefromSlot _save_slot_highscore))
        (bind _asbp_highscore_save (Utilities|Casting|CastToBP_HighscoreSave _returnvalue_7))
        (Variables|Default|SetSaveFileHighscore _asbp_highscore_save)
        (else
          (bind _returnvalue_8 (SaveGame|CreateSaveGameObject "/Game/InfiniteMatrix/Blueprints/BP_HighscoreSave.BP_HighscoreSave_C"))
          (Variables|Default|SetSaveFileHighscore _returnvalue_8)))
      (CallFunction|LoadHighscore)
      (Default|UpdateHighscore (Variables|Default|GetHUD_Widget)))
    (:then_5
      ;[1 1 1] Биндим эвент у игрока когда он столкнется со стеной с функцией вызова геймовера
      (EventDispatchers|BindEventtoHitWall (Variables|Default|GetPlayer) (delegate Custom|CustomEvent_0)))
    (:then_6
      ;[1 1 1] Загружаем настройки звуков и музыки и применяем их для этого уровня (MainLevel)
      (Class|GameplayStatics|SetBaseSoundMix "/Game/InfiniteMatrix/Sounds/S_Volume_Mix.S_Volume_Mix")
      (bind _returnvalue_9 (SaveGame|DoesSaveGameExist _save_slot_settings))
      (if _returnvalue_9
        (bind _returnvalue_10 (SaveGame|LoadGamefromSlot _save_slot_settings))
        (else
          (SaveGame|CreateSaveGameObject "/Game/InfiniteMatrix/Blueprints/BP_SettingsSave.BP_SettingsSave_C")))
      (bind _asbp_settings_save (Utilities|Casting|CastToBP_SettingsSave _returnvalue_10))
      (Audio|SetSoundMixClassOverride "/Game/InfiniteMatrix/Sounds/S_Volume_Mix.S_Volume_Mix" "/Game/InfiniteMatrix/Sounds/S_Music_Class.S_Music_Class" (Variables|/Game/InfiniteMatrix/Blueprints/BP_SettingsSave.BP_SettingsSave_C|GetVolumeMusic _asbp_settings_save) 1.0 0.0 true)
      (Audio|SetSoundMixClassOverride "/Game/InfiniteMatrix/Sounds/S_Volume_Mix.S_Volume_Mix" "/Game/InfiniteMatrix/Sounds/S_Sounds_Class.S_Sounds_Class" (Variables|/Game/InfiniteMatrix/Blueprints/BP_SettingsSave.BP_SettingsSave_C|GetVolumeSounds _asbp_settings_save) 1.0 0.0 true))))

(event Input|KeyboardEvents|Escape
  (params (Key :type Key%20Structure :default "None"))
  ;[1 1 1] Вызов паузы на Q. Возврат из меню настроек в меню паузы
  (:Pressed
    (if (Variables|Default|GetIsPaused)
      (if (Variables|Default|GetIsOptionsMenu)
        (Development|PrintString "pause" :!label _label)
        (CallFunction|OpenPauseMenu)
        (else
          (Development|PrintString "unpause")
          (CallFunction|UnpauseGame)))
      (else
        (goto _label)))))

(fn ConstructionScript)

(fn ResetScore
  (bind _ref_bptunnelspawner_bpgamemanager (Variables|Default|GetRef_BPTunnelSpawner_BPGameManager))
  ;[1 1 1] Обнуление счета и отображение на экране
  (Variables|Default|SetScore 0)
  (Variables|Default|SetLevel 1)
  (Variables|Default|SetScoresPerLevel 5)
  (Default|UpdateScore (Variables|Default|GetHUD_Widget))
  ;[1 1 1] возврат начальной скорости игрока
  (Variables|/Game/InfiniteMatrix/Blueprints/BP_Player.BP_Player_C|SetMoveForward (Variables|Default|GetPlayer) 1e+03)
  ;[1 1 1] Возврат начальной скорости вращения стенок
  (Utilities|IsValid _ref_bptunnelspawner_bpgamemanager
    (:Is%20Valid
      (Variables|/Game/InfiniteMatrix/Blueprints/BP_TunnelSpawner.BP_TunnelSpawner_C|SetRotateSpeedForTunnel _ref_bptunnelspawner_bpgamemanager 3e+01))))

(fn IncrementScore
  (bind _player (Variables|Default|GetPlayer))
  (bind _ref_bptunnelspawner_bpgamemanager (Variables|Default|GetRef_BPTunnelSpawner_BPGameManager))
  ;[1 1 1] Увеличиваем счет и проверям переходить ли на след. уровень
  (bind _result (Math|Integer|IncrementInt (Variables|Default|GetScore))
    (:%20%20
      (if (>= _result (Variables|Default|GetScoresPerLevel))
        ;[1 1 1] Повышение уровня
        (Math|Integer|IncrementInt (Variables|Default|GetLevel)
          (:%20%20
            (Variables|Default|SetIsNewLevel true))))
      ;[1 1 1] Обновление виджета
      (Default|UpdateScore (Variables|Default|GetHUD_Widget))
      ;[1 1 1] Если новый уровень - увеличиваем скорость движения игрока. но перед этим увеличиваем значение очков для перехода на след. уровень
      (if (Variables|Default|GetIsNewLevel)
        (Variables|Default|SetIsNewLevel false)
        (CallFunction|IncrementScorePerLevel)
        (Variables|/Game/InfiniteMatrix/Blueprints/BP_Player.BP_Player_C|SetMoveForward _player (+ (Variables|/Game/InfiniteMatrix/Blueprints/BP_Player.BP_Player_C|GetMoveForward _player) (Variables|Default|GetMoveSpeedPerLevel)))
        ;[1 1 1] Увеличиваем скорость вращения стенок
        (Utilities|IsValid _ref_bptunnelspawner_bpgamemanager
          (:Is%20Valid
            (Variables|/Game/InfiniteMatrix/Blueprints/BP_TunnelSpawner.BP_TunnelSpawner_C|SetRotateSpeedForTunnel _ref_bptunnelspawner_bpgamemanager (+ (Variables|/Game/InfiniteMatrix/Blueprints/BP_TunnelSpawner.BP_TunnelSpawner_C|GetRotateSpeedForTunnel _ref_bptunnelspawner_bpgamemanager) (Variables|Default|GetRotateSpeedPerLevel)))))))))

(fn IncrementScorePerLevel
  ;[1 1 1] scoresPerLevel = scoresPerLevel + (level - 1) * moreScoresForNextLevel
  (Variables|Default|SetScoresPerLevel (+ (Variables|Default|GetScoresPerLevel) (* (- (Variables|Default|GetLevel) 1) (Variables|Default|GetMoreScoresForNextLevel)))))

(fn LoadHighscore
  (bind _savefilehighscore (Variables|Default|GetSaveFileHighscore))
  (bind _records (Variables|/Game/InfiniteMatrix/Blueprints/BP_HighscoreSave.BP_HighscoreSave_C|GetRecords _savefilehighscore))
  (bind _output (Utilities|Array|Get(acopy) _records))
  (SaveGame|LoadGamefromSlot (Variables|Default|Getsave_slot_highscore))
  (if (!= (Utilities|Array|Length _records) 0)
    (Variables|Default|SetHighestLevel (.level _output))
    (Variables|Default|SetHighestScore (.score _output))))

(fn OpenPauseMenu
  (bind _returnvalue (Game|GetPlayerController 0))
  (Class|AudioComponent|SetPaused (Variables|Default|GetAudioMainTheme) true)
  (Input|SetInputModeGameandUI _returnvalue 0 "DoNotLock" false)
  (Variables|/Script/Engine.PlayerController|SetbShowMouseCursor _returnvalue true)
  (Variables|/Game/InfiniteMatrix/Blueprints/BP_Player.BP_Player_C|SetIsDead (Variables|Default|GetPlayer) true)
  ;[1 1 1] Останавливаем вращение стенок у всех туннелей (если открыли паузу из игры, а не из опций)
  (if (Variables|Default|GetIsOptionsMenu)
    _
    (else
      (bind _outactors (Actor|GetAllActorsOfClass "/Game/InfiniteMatrix/Blueprints/BP_Tunnel.BP_Tunnel_C"))
      (Variables|Default|SetCurrentRotateSpeed (Variables|/Game/InfiniteMatrix/Blueprints/BP_Tunnel.BP_Tunnel_C|GetRotateSpeed (Utilities|Array|Get(acopy) _outactors)))
      (for _array_element _outactors
        (Variables|/Game/InfiniteMatrix/Blueprints/BP_Tunnel.BP_Tunnel_C|SetRotateSpeed _array_element 0.0))))
  (Variables|Default|SetIsPaused true)
  (Viewport|RemoveAllWidgets)
  (UserInterface|Viewport|AddtoViewport (Variables|Default|GetPauseWidget) 0)
  (Variables|Default|SetIsOptionsMenu false))

(fn UnpauseGame
  (bind _returnvalue (Game|GetPlayerController 0))
  (Class|AudioComponent|SetPaused (Variables|Default|GetAudioMainTheme) false)
  (Input|SetInputModeGameOnly _returnvalue)
  (Variables|/Script/Engine.PlayerController|SetbShowMouseCursor _returnvalue false)
  (Variables|/Game/InfiniteMatrix/Blueprints/BP_Player.BP_Player_C|SetIsDead (Variables|Default|GetPlayer) false)
  ;[1 1 1] Возвращаем врщение стенок
  (bind _outactors (Actor|GetAllActorsOfClass "/Game/InfiniteMatrix/Blueprints/BP_Tunnel.BP_Tunnel_C"))
  (for _array_element _outactors
    (Variables|/Game/InfiniteMatrix/Blueprints/BP_Tunnel.BP_Tunnel_C|SetRotateSpeed _array_element (Variables|Default|GetCurrentRotateSpeed)))
  (Variables|Default|SetIsPaused false)
  (Viewport|RemoveAllWidgets)
  (UserInterface|Viewport|AddtoViewport (Variables|Default|GetHUD_Widget) 0))

(fn RestartGame
  (bind _returnvalue (Game|GetPlayerController 0))
  (bind _audiomaintheme (Variables|Default|GetAudioMainTheme))
  (Viewport|RemoveAllWidgets)
  (UserInterface|Viewport|AddtoViewport (Variables|Default|GetHUD_Widget) 0)
  (Variables|/Game/InfiniteMatrix/Blueprints/BP_Player.BP_Player_C|SetIsDead (Variables|Default|GetPlayer) false)
  (Input|SetInputModeGameOnly _returnvalue)
  (Variables|/Script/Engine.PlayerController|SetbShowMouseCursor _returnvalue false)
  (bind _outactors (Actor|GetAllActorsOfClass "/Game/InfiniteMatrix/Blueprints/BP_TunnelSpawner.BP_TunnelSpawner_C"))
  (Default|SpawnSeveralTunnels (Utilities|Array|Get(acopy) _outactors))
  (Variables|Default|SetIsPaused false)
  (Class|AudioComponent|SetPaused _audiomaintheme false)
  (Audio|Components|Audio|Play _audiomaintheme 0.0))

(fn GameOver
  (bind _returnvalue (Game|GetPlayerController 0))
  (bind _returnvalue_2 (Math|DateTime|Now))
  (bind _savefilehighscore (Variables|Default|GetSaveFileHighscore))
  (bind _gameoverwidget (Variables|Default|GetGameOverWidget))
  (bind _records (Variables|/Game/InfiniteMatrix/Blueprints/BP_HighscoreSave.BP_HighscoreSave_C|GetRecords _savefilehighscore))
  ;[1 1 1] Останавливаем вращение стенок
  (bind _outactors (Actor|GetAllActorsOfClass "/Game/InfiniteMatrix/Blueprints/BP_Tunnel.BP_Tunnel_C"))
  (for _array_element _outactors
    (Variables|/Game/InfiniteMatrix/Blueprints/BP_Tunnel.BP_Tunnel_C|SetRotateSpeed _array_element 0.0))
  ;[1 1 1] Сначала проверяем не пустой ли массив с рекордами. если пустой, то пропускаем все и сразу вставляем текущий счет. Далее, если текущий счет меньше самого худшего хайскора и уже превышен лимит, то не добавляем его (нод где print skip)
  (bind _output_get (LocalVariables|Setrecords_size (Utilities|Array|Length _records)))
  (if (== _output_get 0)
    ;[1 1 1] Ищем куда вставить текущий рекорд чтобы сохранить сортировку по очкам
    (Utilities|Array|Insert _records (Utilities|Struct|MakeStructure_Highscore (Variables|Default|GetLevel) (Variables|Default|GetScore) (Utilities|String|Append (Utilities|String|ToString(Integer) (.day _returnvalue_2)) "/" (Utilities|String|ToString(Integer) (.month _returnvalue_2)) "/" (Utilities|String|ToString(Integer) (.year _returnvalue_2)) " " (Utilities|String|ToString(Integer) (.hour _returnvalue_2)) ":" (Utilities|String|ToString(Integer) (.minute _returnvalue_2)) ":" (Utilities|String|ToString(Integer) (.second _returnvalue_2)))) (LocalVariables|Getindex_insert) :!label _label)
    ;[1 1 1] Если превышено макс. количество сохраненных рекордов то удаляем последний
    (if (> (Utilities|Array|Length _records) (Variables|Default|GetMaxRecordsInList))
      (Utilities|Array|RemoveIndex (Variables|/Game/InfiniteMatrix/Blueprints/BP_HighscoreSave.BP_HighscoreSave_C|GetRecords (Variables|Default|GetSaveFileHighscore)) (LocalVariables|Getrecords_size))
      (Development|PrintString "deleted last record")
      (else
        (Development|PrintString "new record")))
    (SaveGame|SaveGametoSlot _savefilehighscore (Variables|Default|Getsave_slot_highscore))
    ;[1 1 1] Если был установлен новый найлучший рекорд то обновляем переменные
    (if (== (LocalVariables|Getindex_insert) 0)
      (Variables|Default|SetHighestScore (Variables|Default|GetScore))
      (Variables|Default|SetHighestLevel (Variables|Default|GetLevel))
      (Default|UpdateHighscore (Variables|Default|GetHUD_Widget))
      (Variables|/Game/InfiniteMatrix/UI/WBP_GameOverMenu.WBP_GameOverMenu_C|SetIsNewRecord (Variables|Default|GetGameOverWidget) true))
    ;[1 1 1] Убираем все виджеты, показываем виджет с геймовером, устанавливаем на нем текущей счет, ставим UI mode, показываем курсор мыши, останавливаем музыку
    (Viewport|RemoveAllWidgets)
    (UserInterface|Viewport|AddtoViewport _gameoverwidget 0)
    (Default|SetScore _gameoverwidget)
    (Input|SetInputModeUIOnly _returnvalue 0 "DoNotLock")
    (Variables|/Script/Engine.PlayerController|SetbShowMouseCursor _returnvalue true)
    (Audio|Components|Audio|Stop (Variables|Default|GetAudioMainTheme))
    (elif (and (== 0 (Variables|Default|GetMaxRecordsInList)) (>= (.score (Utilities|Array|Get(acopy) _records (- _output_get 1))) (Variables|Default|GetScore)))
      (Development|PrintString "skip")
      (else
        (bind _index (Utilities|FlowControl|ForLoopwithBreak 0 (- _output_get 1) :!label _label_2)
          (:LoopBody
            (if (or (< _index 0) (>= _index (LocalVariables|Getrecords_size)))
              (goto _label_2 Break)
              (elif (<= (Variables|Default|GetScore) (.score (Utilities|Array|Get(acopy) _records _index)))
                (Math|Integer|IncrementInt (LocalVariables|Getindex_insert))
                (else
                  (goto _label_2 Break)))))
          (:Completed
            (goto _label)))))))

(fn OpenOptionsMenu
  (bind _optionswidget (Variables|Default|GetOptionsWidget))
  (Viewport|RemoveAllWidgets)
  (UserInterface|Viewport|AddtoViewport _optionswidget 0)
  (Variables|Default|SetIsOptionsMenu true)
  (Variables|/Game/InfiniteMatrix/UI/WBP_OptionsMenu.WBP_OptionsMenu_C|SetIsMainMenu _optionswidget false))