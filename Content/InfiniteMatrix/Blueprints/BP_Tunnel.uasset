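; BP_Tunnel is a tunnel segment with a spinning holed wall that serves as an obstacle for the player.
; RandomizeWall picks one of four hole meshes and gives it a random roll and color.
; Passing the trigger zone asks the tunnel spawner for a new segment and destroys this one.
; Hitting the wall marks BP_Player dead, calls its hit-wall handler and plays a sound.
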(event OnComponentBeginOverlap(Trigger_zone)
  (params (OverlappedComponent :type Primitive%20Component%20Object%20Reference) (OtherActor :type Actor%20Object%20Reference) (OtherComp :type Primitive%20Component%20Object%20Reference) (OtherBodyIndex :type Integer) (bFromSweep :type Boolean) (SweepResult :type Hit%20Result%20Structure%20%28by%20ref%29))
  ;[1 1 1] Проход через триггер зону игроком
  (Utilities|Casting|CastToBP_Player OtherActor)
  (Default|SpawnTunnelatSpawnPoint (Variables|Default|GetRef_BP_TunnelSpawner))
  (Actor|DestroyActor))

(event OnComponentHit(WallMesh)
  (params (HitComponent :type Primitive%20Component%20Object%20Reference) (OtherActor :type Actor%20Object%20Reference) (OtherComp :type Primitive%20Component%20Object%20Reference) (NormalImpulse :type Vector :default "0, 0, 0") (Hit :type Hit%20Result%20Structure%20%28by%20ref%29))
  ;[1 1 1] Столкновение со стеной
  (bind _asbp_player (Utilities|Casting|CastToBP_Player OtherActor))
  (Variables|/Game/InfiniteMatrix/Blueprints/BP_Player.BP_Player_C|SetIsDead _asbp_player true)
  (Default|CallHitWall _asbp_player)
  (Audio|PlaySound2D "/Game/InfiniteMatrix/Sounds/Sound_Hit.Sound_Hit" 1.0 1.0 0.0 0 0))

(event EventTick
  (params (DeltaSeconds :type Float%20%28single-precision%29))
  ;[1 1 1] Вращение стенки
  (Transformation|AddLocalRotation (Variables|Default|GetWallMesh) (Math|Rotator|MakeRotator (* DeltaSeconds (Variables|Default|GetRotateSpeed)) 0.0 0.0) false false))

(fn ConstructionScript)

(fn RandomizeWall
  (bind _wallmesh (Variables|Default|GetWallMesh))
  ;[1 1 1] Случайный выбор стенки для туннеля
  (Components|StaticMesh|SetStaticMesh (Variables|Default|GetWallMesh) (Utilities|Select :Index (Math|Random|RandomIntegerinRange 0 3) :Option%200 "/Game/InfiniteMatrix/Meshes/SM_Hole_01_Origin.SM_Hole_01_Origin" :Option%201 "/Game/InfiniteMatrix/Meshes/SM_Hole_02_Origin.SM_Hole_02_Origin" :Option%202 "/Game/InfiniteMatrix/Meshes/SM_Hole_03_Origin.SM_Hole_03_Origin" :Option%203 "/Game/InfiniteMatrix/Meshes/SM_Hole_04_Origin.SM_Hole_04_Origin"))
  (Transformation|AddLocalRotation _wallmesh (Math|Rotator|MakeRotator (Math|Random|RandomFloatinRange 0.0 3.6e+02) 0.0 0.0) false false)
  ;[1 1 1] Зададим случайны цвет для стенки
  (Rendering|Material|SetVectorParameterValueonMaterials _wallmesh "Color" (Math|Conversions|ToVector(LinearColor) (Utilities|Struct|MakeLinearColor (Math|Random|RandomFloatinRange 0.0 1.0) (Math|Random|RandomFloatinRange 0.0 1.0) (Math|Random|RandomFloatinRange 0.0 1.0) 1.0))))